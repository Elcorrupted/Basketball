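; HillTileBP is a hill ground tile that may start covered in snow, which a physics ball can pick up.
; On BeginPlay a coin-flip sets the Snow flag and, if true, applies the snow material to Ground.
; When a PhysicsBallBP overlaps the Box on a snowy tile, it calls GatherSnow on the ball, clears the flag and switches Ground to grass.
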(event `self.ReceiveBeginPlay`
  (bind _output_get (set `self.Snow` (== (`KismetMathLibrary.RandomInteger` 2) 0)))
  (if _output_get
    (`PrimitiveComponent.SetMaterial` (`self.Ground`) 0 "/Game/CustomContent/Materials/M_Snow.M_Snow")))

(event `self.ReceiveActorBeginOverlap`
  (params (OtherActor :type "Actor Object Reference")))

(event `self.Box.OnComponentBeginOverlap`
  (params (OverlappedComponent :type "PrimitiveComponent Object Reference") (OtherActor :type "Actor Object Reference") (OtherComp :type "PrimitiveComponent Object Reference") (OtherBodyIndex :type Integer) (bFromSweep :type Boolean) (SweepResult :type "HitResult Structure (by ref)"))
  (bind _asphysics_ball_bp (cast `/Game/RollingBP/Blueprints/PhysicsBallBP` OtherActor))
  (if (`self.Snow`)
    (`/Game/RollingBP/Blueprints/PhysicsBallBP.GatherSnow` _asphysics_ball_bp)
    (set `self.Snow` false)
    (`PrimitiveComponent.SetMaterial` (`self.Ground`) 0 "/Game/StarterContent/Materials/M_Ground_Grass.M_Ground_Grass")))

(fn `UserConstructionScript`)